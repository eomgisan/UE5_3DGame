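; BP_Plane is a plane that flies forward continuously and is steered through axis input.
; Tick moves the actor along its forward vector by MoveSpeed each frame, without delta-time scaling or collision sweep.
; The UpDown, FrontBack and LeftRight axes apply inverted local roll, pitch and yaw rotations to the Body component, also per frame.
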(event EventBeginPlay)

(event Collision|EventActorBeginOverlap
  (params (OtherActor :type Actor%20Object%20Reference)))

(event EventTick
  (params (DeltaSeconds :type Float%20%28single-precision%29))
  (Transformation|SetActorLocation (+ (Transformation|GetActorLocation) (* (Transformation|GetActorForwardVector) (* "1.000000,1.000000,1.000000" (Variables|Default|GetMoveSpeed)))) false false))

(event Input|AxisEvents|InputAxisUpDown
  (params (AxisValue :type Float%20%28single-precision%29))
  (if (!= AxisValue 0.0)
    (Transformation|AddLocalRotation (Variables|Default|GetBody) (Math|Rotator|MakeRotator (* AxisValue -1.0) 0.0 0.0) false false)))

(event Input|AxisEvents|InputAxisFrontBack
  (params (AxisValue :type Float%20%28single-precision%29))
  (if (!= AxisValue 0.0)
    (Transformation|AddLocalRotation (Variables|Default|GetBody) (Math|Rotator|MakeRotator 0.0 (* AxisValue -1.0) 0.0) false false)))

(event Input|AxisEvents|InputAxisLeftRight
  (params (AxisValue :type Float%20%28single-precision%29))
  (if (!= AxisValue 0.0)
    (Transformation|AddLocalRotation (Variables|Default|GetBody) (Math|Rotator|MakeRotator 0.0 0.0 (* AxisValue -1.0)) false false)))

(fn ConstructionScript)